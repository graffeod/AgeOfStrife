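; Player controller for a vehicle that handles mouse-driven firing and a manual hit on the controlled car.
; Holding left mouse opens a Tick-fed gate into a short Delay, repeatedly spawning Basic actors above the pawn.
; Each spawn is rotated toward the world point under the cursor.
; Right mouse calls VehicleHit with a fixed value on the possessed BasicCarBP.
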(event EventTick
  (params (DeltaSeconds :type Float%20%28single-precision%29))
  (bind _returnvalue (Pawn|GetControlledPawn))
  (bind _returnvalue_2 (Transformation|GetActorLocation _returnvalue))
  (Utilities|FlowControl|Gate true
    (:Exit
      (Utilities|FlowControl|Delay 0.1)
      (Game|SpawnActorfromClass "/Game/AoS/Blueprints/Ammo/Basic.Basic_C" (Math|Transform|MakeTransform (+ _returnvalue_2 "0.000000,0.000000,200.000000") (Math|Rotator|FindLookatRotation _returnvalue_2 (.Location (Collision|BreakHitResult (.HitResult (Game|Player|GetHitResultUnderCursorbyChannel "TraceTypeQuery1" true))))) "1,1.000000,1") "AlwaysSpawn" 0 0))))

(event Input|MouseEvents|LeftMouseButton
  (params (Key :type Key%20Structure :default "AnyKey"))
  (bind _returnvalue (Pawn|GetControlledPawn))
  (bind _returnvalue_2 (Transformation|GetActorLocation _returnvalue))
  (:Pressed
    (Utilities|FlowControl|Gate true) ; enters at Open
  )
  (:Released
    (Utilities|FlowControl|Gate true) ; enters at Close
  ))

(event Input|MouseEvents|RightMouseButton
  (params (Key :type Key%20Structure :default "AnyKey"))
  (:Pressed
    (bind _asbasic_car_bp (Utilities|Casting|CastToBasicCarBP (Pawn|GetControlledPawn)))
    (Default|VehicleHit _asbasic_car_bp 0.25)))

(fn ConstructionScript)